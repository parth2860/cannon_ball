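; Base game mode Blueprint that reacts to a test event dispatcher on the player character.
; On BeginPlay it casts player character 0 to char_bp and binds its own handler to that dispatcher.
; The handler prints a debug "Hello" when the character's player-state component reports level 2.
; Disconnected DoOnce and health-increase nodes remain in the graph but never run.
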(event `self.ReceiveBeginPlay`
  (bind _aschar_bp (cast `/Game/blueprint/char_bp` (`GameplayStatics.GetPlayerCharacter` 0)))
  (add `/Game/blueprint/char_bp.test_event` _aschar_bp (delegate `test_event_Event`)))

(event `test_event_Event`
  (if (== (`/Game/blueprint/charcter/bpc_playerstate.level` (`/Game/blueprint/char_bp.bpc_playerstate` (stale `self.ReceiveBeginPlay` _aschar_bp))) 2)
    (`KismetSystemLibrary.PrintString` "Hello")))

(fn `UserConstructionScript`)