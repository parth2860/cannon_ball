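; Player stats component for char_bp that tracks health, stamina, XP, level and score.
; On BeginPlay it waits a tick, caches its owner and fills the HUD, then each change function writes directly to that HUD.
; Decrease functions return whether the stat is depleted, and reaching max XP levels up, resetting XP and raising its cap.
; Every fifth level raises max health and stamina, though the max stamina update sets its bar from the health ratio.
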(event `self.ReceiveBeginPlay`
  (`KismetSystemLibrary.DelayUntilNextTick`)
  (bind _aschar_bp (cast `/Game/blueprint/char_bp` (`self.GetOwner`)))
  (set `self.As Char Bp` _aschar_bp)
  (`ProgressBar.SetPercent` (`/Game/blueprint/hud/bp_ui_hud.stamina` (`/Game/blueprint/char_bp.hud_widget` (`self.As Char Bp`))) (/ (`self.current_stamina`) (`self.max_stamina`)))
  (`ProgressBar.SetPercent` (`/Game/blueprint/hud/bp_ui_hud.health` (`/Game/blueprint/char_bp.hud_widget` (`self.As Char Bp`))) (/ (`self.current_health`) (`self.max_health`)))
  (`ProgressBar.SetPercent` (`/Game/blueprint/hud/bp_ui_hud.xp_bar` (`/Game/blueprint/char_bp.hud_widget` (`self.As Char Bp`))) (/ (`self.xp`) (`self.max_xp`)))
  (`TextBlock.SetText` (`/Game/blueprint/hud/bp_ui_hud.xp_text` (`/Game/blueprint/char_bp.hud_widget` (`self.As Char Bp`))) (`|FormatText` "{current_xp}/{max_xp}" (`self.xp`) (`self.max_xp`)))
  (`TextBlock.SetText` (`/Game/blueprint/hud/bp_ui_hud.level_text` (`/Game/blueprint/char_bp.hud_widget` (`self.As Char Bp`))) (`KismetTextLibrary.Conv_IntToText` (`self.level`)))
  (`TextBlock.SetText` (`/Game/blueprint/hud/bp_ui_hud.score` (`/Game/blueprint/char_bp.hud_widget` (`self.As Char Bp`))) (`KismetTextLibrary.Conv_DoubleToText` (`self.score`) "HalfToEven")))

(fn `Decrease Health`
  (params (damage :type "Float (double-precision)"))
  (returns (player_dead :type Boolean))
  (bind _hud_widget (`/Game/blueprint/char_bp.hud_widget` (`self.As Char Bp`)))
  (if (not (<= (`self.current_health`) 0.0))
    (bind _output_get (set `self.current_health` (- (`self.current_health`) damage)))
    (`ProgressBar.SetPercent` (`/Game/blueprint/hud/bp_ui_hud.health` _hud_widget) (/ _output_get (`self.max_health`)))
    (`TextBlock.SetText` (`/Game/blueprint/hud/bp_ui_hud.health_text` _hud_widget) (`KismetTextLibrary.Conv_DoubleToText` (`self.current_health`) "HalfToEven"))
    (if (<= (`self.current_health`) 0.0)
      _
      (else
        (return false))))
  (return true))

(fn `decrease_stamina`
  (params (`stamina-` :type "Float (double-precision)"))
  (returns (not_stamina_left :type Boolean))
  (if (not (<= (`self.current_stamina`) 0.0))
    (set `self.current_stamina` (- (`self.current_stamina`) `stamina-`))
    (`ProgressBar.SetPercent` (`/Game/blueprint/hud/bp_ui_hud.stamina` (`/Game/blueprint/char_bp.hud_widget` (`self.As Char Bp`))) (/ (`self.current_stamina`) (`self.max_stamina`)))
    (if (<= (`self.current_stamina`) 0.0)
      _
      (else
        (return false))))
  (return true))

(fn `increase_health`
  (params (`health+` :type "Float (double-precision)"))
  (bind _hud_widget (`/Game/blueprint/char_bp.hud_widget` (`self.As Char Bp`)))
  (set `self.current_health` (+ (`self.current_health`) `health+`))
  (if (>= (`self.current_health`) (`self.max_health`))
    (set `self.current_health` (`self.max_health`)))
  (`ProgressBar.SetPercent` (`/Game/blueprint/hud/bp_ui_hud.health` _hud_widget) (/ (`self.current_health`) (`self.max_health`)))
  (`TextBlock.SetText` (`/Game/blueprint/hud/bp_ui_hud.health_text` _hud_widget) (`KismetTextLibrary.Conv_DoubleToText` (`self.current_health`) "HalfToEven")))

(fn `increase_level`
  (params (`level+` :type Integer))
  (`|ExecutionSequence`
    (:`then_0`
      (set `self.level` (+ (`self.level`) `level+`))
      (set `self.max_xp` (+ (`self.max_xp`) 150.0))
      (set `self.xp` 0.0)
      (`TextBlock.SetText` (`/Game/blueprint/hud/bp_ui_hud.level_text` (`/Game/blueprint/char_bp.hud_widget` (`self.As Char Bp`))) (`KismetTextLibrary.Conv_IntToText` (`self.level`))))
    (:`then_1`
      ;[1 1 1] every 5 level max and stamina increase
      (if (== (mod (`self.level`) 5) 0)
        (`self.increase_max_stamina` 10.0)
        (`self.increase_max_health` 10.0)))))

(fn `increase_max_health`
  (params (`health+` :type "Float (double-precision)"))
  (bind _hud_widget (`/Game/blueprint/char_bp.hud_widget` (`self.As Char Bp`)))
  (set `self.max_health` (+ (`self.max_health`) `health+`))
  (`ProgressBar.SetPercent` (`/Game/blueprint/hud/bp_ui_hud.health` _hud_widget) (/ (`self.current_health`) (`self.max_health`)))
  (`TextBlock.SetText` (`/Game/blueprint/hud/bp_ui_hud.health_text` _hud_widget) (`KismetTextLibrary.Conv_DoubleToText` (`self.current_health`) "HalfToEven")))

(fn `increase_max_stamina`
  (params (`stamina+` :type "Float (double-precision)"))
  (set `self.max_stamina` (+ (`self.max_stamina`) `stamina+`))
  (`ProgressBar.SetPercent` (`/Game/blueprint/hud/bp_ui_hud.stamina` (`/Game/blueprint/char_bp.hud_widget` (`self.As Char Bp`))) (/ (`self.current_health`) (`self.max_health`))))

(fn `increase_score`
  (params (`score+` :type "Float (double-precision)"))
  (set `self.score` (+ (`self.score`) `score+`))
  (`TextBlock.SetText` (`/Game/blueprint/hud/bp_ui_hud.score` (`/Game/blueprint/char_bp.hud_widget` (`self.As Char Bp`))) (`KismetTextLibrary.Conv_DoubleToText` (`self.score`) "HalfToEven")))

(fn `increase_stamina`
  (params (`stamina+` :type "Float (double-precision)"))
  (set `self.current_stamina` (+ (`self.current_stamina`) `stamina+`))
  (if (> (`self.current_stamina`) (`self.max_stamina`))
    (set `self.current_stamina` (`self.max_stamina`)))
  (`ProgressBar.SetPercent` (`/Game/blueprint/hud/bp_ui_hud.stamina` (`/Game/blueprint/char_bp.hud_widget` (`self.As Char Bp`))) (/ (`self.current_stamina`) (`self.max_stamina`))))

(fn `increase_xp`
  (params (`xp+` :type "Float (double-precision)"))
  (set `self.xp` (+ (`self.xp`) `xp+`))
  (if (>= (`self.xp`) (`self.max_xp`))
    (`self.increase_level` 1))
  (`ProgressBar.SetPercent` (`/Game/blueprint/hud/bp_ui_hud.xp_bar` (`/Game/blueprint/char_bp.hud_widget` (`self.As Char Bp`))) (/ (`self.xp`) (`self.max_xp`)))
  (`TextBlock.SetText` (`/Game/blueprint/hud/bp_ui_hud.xp_text` (`/Game/blueprint/char_bp.hud_widget` (`self.As Char Bp`))) (`|FormatText` "{current_xp}/{max_xp}" (`self.xp`) (`self.max_xp`))))