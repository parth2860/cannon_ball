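; Coin pickup actor that awards score to the player when the char_bp character touches it.
; A Sphere overlap with char_bp calls AddScore, which adds a fixed amount to the Score variable on player 0's character.
; It then plays a coin sound, spawns an auto-released pickup particle system at its location and destroys itself.
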(event `self.ReceiveActorBeginOverlap`
  (params (OtherActor :type "Actor Object Reference"))
  ;[1 1 1] score
)

(event `add score`
  ;[1 1 1] score
  (bind _aschar_bp (cast `/Game/blueprint/char_bp` (`GameplayStatics.GetPlayerCharacter` 0)))
  (set `/Game/blueprint/char_bp.score` (+ (`/Game/blueprint/char_bp.score` _aschar_bp) 100) _aschar_bp))

(event `self.Sphere.OnComponentBeginOverlap`
  (params (OverlappedComponent :type "PrimitiveComponent Object Reference") (OtherActor :type "Actor Object Reference") (OtherComp :type "PrimitiveComponent Object Reference") (OtherBodyIndex :type Integer) (bFromSweep :type Boolean) (SweepResult :type "HitResult Structure (by ref)"))
  (bind _returnvalue (`self.K2_GetActorLocation`))
  ;[1 1 1] pickup action scene
  (cast `/Game/blueprint/char_bp` OtherActor)
  (`self.add score`)
  (`GameplayStatics.PlaySoundAtLocation` "/Game/blueprint/collectable/341695__projectsu012__coins-1.341695__projectsu012__coins-1" _returnvalue (struct) 1.0 1.0 0.0 null null null null)
  (`NiagaraFunctionLibrary.SpawnSystemAtLocation` "/Game/blueprint/collectable/coin_pickup_effect.coin_pickup_effect" _returnvalue (struct) (1.0 1.0 1.0) true true "AutoRelease")
  (`self.K2_DestroyActor`))

(fn `UserConstructionScript`)