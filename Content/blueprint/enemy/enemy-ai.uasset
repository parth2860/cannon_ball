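; Enemy AI Blueprint that chases the player once it spots a pawn and damages them on contact.
; PawnSensing sets a seeing flag, never cleared here, and triggers an AI Move To targeting the first player's character.
; Capsule hits on the player character call DecreaseHealth on its player state component.
; An older direct clamped health subtraction remains as unconnected nodes.
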(event `self.PawnSensing.OnSeePawn`
  (params (Pawn :type "Pawn Object Reference"))
  ;[1 1 1] enemy sense
  (set `self.is_seeing` true)
  (`self.enemy follow`))

(event `enemy follow`
  ;[1 1 1] enemy follow
  (if (`self.is_seeing`)
    (`|AIMoveTo` self (0.0 0.0 0.0) (`GameplayStatics.GetPlayerCharacter` 0))))

(event `self.CapsuleComponent.OnComponentHit`
  (params (HitComponent :type "PrimitiveComponent Object Reference") (OtherActor :type "Actor Object Reference") (OtherComp :type "PrimitiveComponent Object Reference") (NormalImpulse :type "Vector Structure") (Hit :type "HitResult Structure (by ref)"))
  ;[1 1 1] enemy interaction
  (bind _aschar_bp (cast `/Game/blueprint/char_bp` OtherActor))
  (`/Game/blueprint/charcter/bpc_playerstate.Decrease Health` (`/Game/blueprint/char_bp.bpc_playerstate` _aschar_bp) 20.0))

(event `self.CapsuleComponent.OnComponentBeginOverlap`
  (params (OverlappedComponent :type "PrimitiveComponent Object Reference") (OtherActor :type "Actor Object Reference") (OtherComp :type "PrimitiveComponent Object Reference") (OtherBodyIndex :type Integer) (bFromSweep :type Boolean) (SweepResult :type "HitResult Structure (by ref)"))
  ;[1 1 1] enemy interaction
)

(fn `UserConstructionScript`)