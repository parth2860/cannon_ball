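; Level spawner actor that alternately spawns obstacles and pickups at the location of its SpawPoint component.
; BeginPlay starts a looping timer that fires the spawn event every few seconds.
; A FlipFlop in that event switches between Bp_obsratcle and Bp_pickup on each firing.
; Each spawned actor is destroyed by the spawner after a random delay, so it exists only briefly.
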(event `self.ReceiveBeginPlay`
  (`KismetSystemLibrary.K2_SetTimerDelegate` (delegate `spawn_event`) 5.0 true))

(event `self.ReceiveTick`
  (params (DeltaSeconds :type "Float (single-precision)")))

(event `spawn_event`
  (bind _returnvalue (`KismetMathLibrary.RandomFloatInRange` 2.7 6.7))
  (`/Engine/EditorBlueprintResources/StandardMacros.FlipFlop`
    (:`A`
      (bind _returnvalue_2 (`|SpawnActorFromClass` "/Game/blueprint/bp_obsratcle.bp_obsratcle_C" (`KismetMathLibrary.Conv_VectorToTransform` (`SceneComponent.K2_GetComponentLocation` (`self.spaw_point`))) "Undefined" "MultiplyWithRoot" null null))
      (`KismetSystemLibrary.Delay` _returnvalue)
      (`self.K2_DestroyActor` _returnvalue_2))
    (:`B`
      (bind _returnvalue_3 (`|SpawnActorFromClass` "/Game/blueprint/bp_pickup.bp_pickup_C" (`KismetMathLibrary.Conv_VectorToTransform` (`SceneComponent.K2_GetComponentLocation` (`self.spaw_point`))) "Undefined" "MultiplyWithRoot" null null))
      (`KismetSystemLibrary.Delay` _returnvalue)
      (`self.K2_DestroyActor` _returnvalue_3))))

(fn `UserConstructionScript`)